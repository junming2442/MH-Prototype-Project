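; Weapon manager component for MH characters that equips and unequips weapon actors, toggling off when the same class is equipped again.
; On authority it spawns the weapon and attaches it to its configured mesh socket.
; The EquippedWeapon RepNotify applies the weapon's anim class, walk speed and wielding GameplayEffect, or restores unarmed defaults cached at BeginPlay.
; Ability granting and rotation settings are present but disconnected.
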(event `self.ReceiveBeginPlay`
  ; BeginPlay
  (bind _asmhcharacter_base (cast `MHCharacterBase` (`self.GetOwner`)))
  (bind _output_get (set `self.CharacterRef` _asmhcharacter_base))
  (bind _charactermovement (`Character.CharacterMovement` _output_get))
  (set `self.DefaultWeaponConfig` (make `/Game/Core/Weapon/Data/F_WeaponConfig` "None" (`SkeletalMeshComponent.AnimClass` (`Character.Mesh` _output_get)) (make `/Game/Core/Weapon/Data/F_MovementProperties` (`CharacterMovementComponent.MaxWalkSpeed` _charactermovement) (`CharacterMovementComponent.bOrientRotationToMovement` _charactermovement) (`CharacterMovementComponent.bUseControllerDesiredRotation` _charactermovement)))))

(event `EquipWeapon`
  (params (WeaponClass :type "/Game/Core/Weapon/BP_WeaponBase Class Reference"))
  ; Equip weapon
  (`/Engine/EditorBlueprintResources/ActorComponentMacros.Switch Has Authority`
    (:`Authority`
      (`self.CharacterRef`
        (:`then`
          (`self.OnWeaponChanged`)
          (bind _equippedweapon (`self.EquippedWeapon`)
            (:`then`
              (if (== (`GameplayStatics.GetObjectClass` _equippedweapon) WeaponClass)
                (`self.UnequipWeapon`)
                (else
                  (`self.UnequipWeapon`)
                  (bind _returnvalue (`|SpawnActorFromClass` WeaponClass (`KismetMathLibrary.MakeTransform` (0.0 0.0 0.0)) "Undefined" "MultiplyWithRoot" null (`self.CharacterRef`) :!label _label))
                  (bind _output_get (set `self.EquippedWeapon` _returnvalue))
                  (`Actor.K2_AttachToComponent` _output_get (`Character.Mesh` (`self.CharacterRef`)) (`.EquippedSocketName_7_27043E1C44F82D161A825395BA5A5913` (break `/Game/Core/Weapon/Data/F_WeaponConfig` (`/Game/Core/Weapon/BP_WeaponBase.WeaponConfig` _output_get))) "SnapToTarget" "SnapToTarget" "SnapToTarget" true))))
            (:`else`
              (goto _label))))
        (:`else`)))))

(event `UnequipWeapon`
  ; Unequip weapon
  (bind _equippedweapon (`self.EquippedWeapon`)
    (:`then`
      (`Actor.K2_DestroyActor` _equippedweapon)
      (set `self.EquippedWeapon` null)
      (`self.SetUnarmedWeaponProperties`))
    (:`else`)))

(event `SetEquippedWeaponProperties`
  ; Set Equip Properties
  (bind _equippedweapon (`self.EquippedWeapon`)
    (:`then`
      (bind ((`AnimClass_10_49ECABF3487B461B7FC6FEA7FE7F1805` _animclass) (`MovementProperties_13_31DB530F4AC3536864CE698CE2914D55` _movementproperties)) (break `/Game/Core/Weapon/Data/F_WeaponConfig` (`/Game/Core/Weapon/BP_WeaponBase.WeaponConfig` _equippedweapon)))
      (`SkeletalMeshComponent.SetAnimInstanceClass` (`Character.Mesh` (`self.CharacterRef`)) _animclass)
      (set `CharacterMovementComponent.MaxWalkSpeed` (`.MaxWalkSpeed_2_8517335A42F62616B07CEC98D55796BB` (break `/Game/Core/Weapon/Data/F_MovementProperties` _movementproperties)) (`Character.CharacterMovement` (`self.CharacterRef`)))
      (`AbilitySystemComponent.BP_ApplyGameplayEffectToSelf` :`self` (`AbilitySystemBlueprintLibrary.GetAbilitySystemComponent` (`self.CharacterRef`)) :`GameplayEffectClass` "/Game/Core/GameplayAbilitySystem/Effects/GE_WieldingWeapon.GE_WieldingWeapon_C"))
    (:`else`)))

(event `SetUnarmedWeaponProperties`
  (bind ((`AnimClass_10_49ECABF3487B461B7FC6FEA7FE7F1805` _animclass) (`MovementProperties_13_31DB530F4AC3536864CE698CE2914D55` _movementproperties)) (break `/Game/Core/Weapon/Data/F_WeaponConfig` (`self.DefaultWeaponConfig`)))
  ; Set Unequip Properties
  (`SkeletalMeshComponent.SetAnimInstanceClass` (`Character.Mesh` (`self.CharacterRef`)) _animclass)
  (set `CharacterMovementComponent.MaxWalkSpeed` (`.MaxWalkSpeed_2_8517335A42F62616B07CEC98D55796BB` (break `/Game/Core/Weapon/Data/F_MovementProperties` _movementproperties)) (`Character.CharacterMovement` (`self.CharacterRef`)))
  (`AbilitySystemComponent.RemoveActiveEffectsWithGrantedTags` (`AbilitySystemBlueprintLibrary.GetAbilitySystemComponent` (`self.CharacterRef`)) (struct :`GameplayTags` (struct :`(TagName` "State.Combat.WieldingWeapon")))))

(fn `OnRep_EquippedWeapon`
  (`self.EquippedWeapon`
    (:`then`
      (`self.SetEquippedWeaponProperties`))
    (:`else`
      (`self.SetUnarmedWeaponProperties`))))