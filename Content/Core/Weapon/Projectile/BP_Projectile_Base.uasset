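; Base GAS projectile actor that launches on BeginPlay with velocity set from TargetLocation times Speed.
; Overlapping a non-instigator destroys it and reports an AI damage event; on authority, targets with an ability system also receive the supplied effect spec and a hardcoded fire debuff.
; Blocking hits also destroy it, and destruction fires the hit gameplay cue; the spawn cue is not wired.
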(event `self.ReceiveBeginPlay`
  (bind _projectilemovement (`self.ProjectileMovement`))
  (set `MovementComponent.Velocity` (* (`self.TargetLocation`) (`self.Speed`)) _projectilemovement)
  (`ActorComponent.Activate` _projectilemovement false))

(event `self.SphereCollision.OnComponentBeginOverlap`
  (params (OverlappedComponent :type "PrimitiveComponent Object Reference") (OtherActor :type "Actor Object Reference") (OtherComp :type "PrimitiveComponent Object Reference") (OtherBodyIndex :type Integer) (bFromSweep :type Boolean) (SweepResult :type "HitResult Structure (by ref)"))
  (bind _returnvalue (`AbilitySystemBlueprintLibrary.GetAbilitySystemComponent` OtherActor))
  (bind _returnvalue_2 (`self.GetInstigator`))
  (if (!= OtherActor (`self.Instigator`))
    (`/Engine/EditorBlueprintResources/StandardMacros.IsValid` _returnvalue
      (:`Is Valid`
        (`/Engine/EditorBlueprintResources/ActorMacros.Switch Has Authority`
          (:`Authority`
            (`AbilitySystemComponent.BP_ApplyGameplayEffectSpecToTarget` (`AbilitySystemBlueprintLibrary.GetAbilitySystemComponent` (`self.GetInstigator`)) (`self.GameplayEffectSpecHandle`) _returnvalue)
            (`AbilitySystemComponent.BP_ApplyGameplayEffectToTarget` :`self` (`AbilitySystemBlueprintLibrary.GetAbilitySystemComponent` (`self.GetInstigator`)) :`GameplayEffectClass` "/Game/Core/GameplayAbilitySystem/Effects/Debuffs/GE_Debuff_Fire.GE_Debuff_Fire_C" :`Target` _returnvalue))
          (:`Remote`
            _)))
      (:`Is Not Valid`
        _))
    (`self.K2_DestroyActor`)
    (`AISense_Damage.ReportDamageEvent` OtherActor _returnvalue_2 10.0 (`self.K2_GetActorLocation` _returnvalue_2))))

(event `self.SphereCollision.OnComponentHit`
  (params (HitComponent :type "PrimitiveComponent Object Reference") (OtherActor :type "Actor Object Reference") (OtherComp :type "PrimitiveComponent Object Reference") (NormalImpulse :type "Vector Structure") (Hit :type "HitResult Structure (by ref)"))
  (`self.K2_DestroyActor`))

(event `self.ReceiveDestroyed`
  (`GameplayCueFunctionLibrary.ExecuteGameplayCueOnActor` self (`self.GameplayCueHit`) (`AbilitySystemBlueprintLibrary.MakeGameplayCueParameters` 0.0 0.0 (struct) (struct) (struct) (struct) (struct) (`self.K2_GetActorLocation`))))

(fn `UserConstructionScript`)