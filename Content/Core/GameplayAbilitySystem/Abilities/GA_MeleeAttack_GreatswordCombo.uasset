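; Greatsword melee combo gameplay ability that extends a parent ability's montage and hit-scan hooks.
; Once the montage starts, parallel gameplay event listeners open and close an input window and record next-combo input.
; At window close the combo count advances if input arrived, otherwise the ability ends; avatars without a player controller always advance.
; Hit-scan damage scales linearly with the combo count.
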(event `self.K2_ActivateAbility`
  (`parent.K2_ActivateAbility`)
  (set `self.IsSingleCombo` (not (`self.HasPlayerController`))))

(event `self.MontageStarted`
  (set `self.ComboCount` 1)
  (`AbilityTask_WaitGameplayEvent.WaitGameplayEvent` (struct :`TagName` "Event.NextCombo.Start") null
    (:`then`
      (`AbilityTask_WaitGameplayEvent.WaitGameplayEvent` (struct :`TagName` "Event.NextCombo.End") null
        (:`then`
          (`AbilityTask_WaitGameplayEvent.WaitGameplayEvent` (struct :`TagName` "Event.NextCombo.Input") null
            (:`EventReceived`
              (set `self.ReceivedInput` (`self.IsWithinComboWindow`)))))
        (:`EventReceived`
          (set `self.IsWithinComboWindow` false)
          (if (or (`self.ReceivedInput`) (`self.IsSingleCombo`))
            (`/Engine/EditorBlueprintResources/StandardMacros.IncrementInt` (`self.ComboCount`))
            (else
              (`self.K2_EndAbility`))))))
    (:`EventReceived`
      (set `self.IsWithinComboWindow` true)
      (set `self.ReceivedInput` false))))

(event `self.HandleHitScanStart`
  (set `self.DamageMagnitude` (* 25.0 (`self.ComboCount`)))
  (`parent.HandleHitScanStart`))