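; Base Gameplay Ability that plays a shoot montage and fires a projectile when the Event.ShootProjectile gameplay event arrives.
; It aims at the avatar's attack target, falling back to instant target data for player-controlled avatars and otherwise ending.
; The projectile spawns on authority at the equipped weapon's spawn point, or the avatar's location, carrying a SetByCaller damage effect spec.
; The ability also ends when the montage completes, is interrupted or is cancelled.
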(event `self.K2_ActivateAbility`
  (`AbilityTask_PlayMontageAndWait.CreatePlayMontageAndWaitProxy` "None" (`self.ShootMontage`) 1.3 "None" true 1.0 0.0 true
    (:`then`
      (`AbilityTask_WaitGameplayEvent.WaitGameplayEvent` (struct :`TagName` "Event.ShootProjectile") null
        (:`EventReceived`
          (bind _attacktarget (message `/Game/Core/Interface/BPI_Targeting.GetAttackTarget` (`self.GetAvatarActorFromActorInfo`)))
          (`/Engine/EditorBlueprintResources/StandardMacros.IsValid` _attacktarget
            (:`Is Valid`
              (`self.ShootProjectile` (`Actor.K2_GetActorLocation` _attacktarget)))
            (:`Is Not Valid`
              (if (`self.HasPlayerController`)
                (bind (_asynctaskproxy _data) (`AbilityTask_WaitTargetData.WaitTargetData` "None" "Instant" "/Script/GameplayAbilities.GameplayAbilityTargetActor_SingleLineTrace" 999999.0 (struct :`Name` "NoCollision") true (`self.MakeTargetLocationInfoFromOwnerActor`) (struct) "" (struct) true)
                  (:`ValidData`
                    (`self.ShootProjectile` (`AbilitySystemBlueprintLibrary.GetTargetDataEndPoint` _data))))
                (else
                  (`self.K2_EndAbility`))))))))
    (:`OnCompleted`
      (`self.K2_EndAbility` :!label _label))
    (:`OnInterrupted`
      (goto _label))
    (:`OnCancelled`
      (goto _label))))

(event `ShootProjectile`
  (params (TargetLocation :type "Vector Structure"))
  (bind _returnvalue (`AbilitySystemBlueprintLibrary.AssignTagSetByCallerMagnitude` (`self.MakeOutgoingGameplayEffectSpec` (`self.DamageEffectClass`)) (struct :`TagName` "Data.Damage") (`self.DamageMagnitude`)))
  (bind _location (`self.GetSpawnLocation`))
  (`GameplayTask_SpawnActor.SpawnActor` null _location (struct) (`self.ProjectileClass`) true (`self.ProjectileSpeed`) TargetLocation _returnvalue (cast `Pawn` (`self.GetAvatarActorFromActorInfo`) :!pure true)))

(fn `GetSpawnLocation`
  (returns (Location :type "Vector Structure"))
  (bind _returnvalue (`Actor.GetComponentByClass` (`self.GetAvatarActorFromActorInfo`) "/Game/Core/Weapon/BP_WeaponManager_Component.BP_WeaponManager_Component_C"))
  (`/Engine/EditorBlueprintResources/StandardMacros.IsValid` _returnvalue
    (:`Is Valid`
      (bind _equippedweapon (`/Game/Core/Weapon/BP_WeaponManager_Component.EquippedWeapon` _returnvalue)
        (:`then`
          (bind _location (`/Game/Core/Weapon/BP_WeaponBase.GetProjectileSpawnLocation` _equippedweapon))
          (if (!= _location (0.0 0.0 0.0))
            (return _location)
            (else
              _)))
        (:`else`
          _)))
    (:`Is Not Valid`
      _))
  (return (`Actor.K2_GetActorLocation` (`self.GetAvatarActorFromActorInfo`))))