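; Base melee attack gameplay ability that plays an attack montage using the avatar's equipped weapon from its weapon manager component.
; On the authority, montage gameplay events start and end the weapon's hit scan, which also ends with the ability.
; Hit scan start passes the weapon a damage effect spec with level-scaled SetByCaller damage, and prints that value.
; Child abilities can override MontageStarted.
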(event Custom|HandleHitScanStart
  (bind _returnvalue (Ability|GetAbilityLevel))
  (bind _damageincreaserate (Variables|GameplayEffect|GetDamageIncreaseRate))
  (bind _returnvalue_2 (Math|Conversions|ToFloat(Integer) _returnvalue))
  (bind _returnvalue_3 (|({2E0F61FD-45F1-5687-4D7E-65A190120EE9}+(({2E0F61FD-45F1-5687-4D7E-65A190120EE9}*Rate)*(AbilityLevel-1))) _returnvalue_2 _damageincreaserate))
  ;[0.15 0.15 0.15 0.5] Hit Scan Events
  (bind _equippedweapon (Variables|Default|GetEquippedWeapon)
    (:then
      (bind _returnvalue_4 (Ability|GameplayEffect|AssignTagSetbyCallerMagnitude (Ability|MakeOutgoingGameplayEffectSpec (Variables|GameplayEffect|GetDamageEffectClass)) "(TagName=\"Data.Damage\")" _returnvalue_3))
      (Default|HitScanStart _equippedweapon _returnvalue_4)
      (Development|PrintString (Utilities|String|ToString(Float) _returnvalue_3)))
    (:else)))

(event Custom|HandleHitScanEnd
  ;[0.15 0.15 0.15 0.5] Hit Scan Events
  (bind _equippedweapon (Variables|Default|GetEquippedWeapon)
    (:then
      (Default|HitScanEnd _equippedweapon))
    (:else)))

(event Custom|MontageStarted
  ;[0.15 0.15 0.15 0.5] Override in child
)

(event Ability|EventActivateAbility
  (bind _returnvalue (Ability|GetAvatarActorfromActorInfo))
  (bind _returnvalue_2 (Actor|GetComponentbyClass _returnvalue "/Game/Core/Weapon/BP_WeaponManager_Component.BP_WeaponManager_Component_C"))
  (Utilities|IsValid _returnvalue_2
    (:Is%20Valid
      (bind _equippedweapon (Variables|/Game/Core/Weapon/BP_WeaponManager_Component.BP_WeaponManager_Component_C|GetEquippedWeapon _returnvalue_2)
        (:then
          (Variables|Default|SetEquippedWeapon _equippedweapon)
          (bind _attackmontage (Variables|Animation|GetAttackMontage)
            (:then
              (|PlayMontageandWaitProxy "None" _attackmontage 1.0 "None" true 1.0 0.0 true
                (:then
                  (CallFunction|MontageStarted)
                  (Ability|HasAuthority
                    (:True
                      (Utilities|FlowControl|Sequence
                        (:then_0
                          (Ability|Tasks|WaitGameplayEvent "(TagName=\"Event.HitScan.Start\")" 0
                            (:EventReceived
                              (CallFunction|HandleHitScanStart))))
                        (:then_1
                          (Ability|Tasks|WaitGameplayEvent "(TagName=\"Event.HitScan.End\")" 0
                            (:EventReceived
                              (CallFunction|HandleHitScanEnd))))))))
                (:OnCompleted
                  (Ability|EndAbility :!label _label))
                (:OnInterrupted
                  (goto _label))
                (:OnCancelled
                  (goto _label))))
            (:else
              (goto _label))))
        (:else
          (goto _label))))
    (:Is%20Not%20Valid
      (goto _label))))

(event Ability|EventOnEndAbility
  (params (bWasCancelled :type Boolean))
  (CallFunction|HandleHitScanEnd))