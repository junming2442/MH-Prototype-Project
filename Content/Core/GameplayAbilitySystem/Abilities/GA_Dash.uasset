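; Gameplay ability that dashes the avatar character along its input acceleration, or its forward vector when there is no acceleration.
; Activation commits the cost, then applies a brief root motion constant force and adds a dash gameplay cue that is removed on end.
; Exit velocity is clamped to the movement component's max speed.
; Cooldown is committed separately when the ability ends, so it starts after the dash.
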(event `self.K2_ActivateAbility`
  (`self.K2_CommitAbilityCost` false)
  (`AbilityTask_ApplyRootMotionConstantForce.ApplyRootMotionConstantForce` "None" (`self.GetDashDirection`) 2000.0 0.3 false null "ClampVelocity" (0.0 0.0 0.0) (`self.GetMaxSpeed`)
    (:`then`
      (`self.K2_AddGameplayCue` (struct :`TagName` "GameplayCue.Dash.Active")))
    (:`OnFinish`
      (`self.K2_EndAbility`))))

(event `self.K2_ActivateAbilityFromEvent`
  (params (EventData :type "GameplayEventData Structure (by ref)")))

(event `self.K2_OnEndAbility`
  (params (bWasCancelled :type Boolean))
  (`self.K2_CommitAbilityCooldown` false))

(fn `GetDashDirection`
  (returns (Direction :type "Vector Structure"))
  (bind _returnvalue (`self.GetAvatarActorFromActorInfo`))
  (bind _ascharacter (cast `Character` _returnvalue)
    (:`then`
      (bind _returnvalue_2 (`CharacterMovementComponent.GetCurrentAcceleration` (`Character.CharacterMovement` _ascharacter)))
      (return (`KismetMathLibrary.SelectVector` _returnvalue_2 (`Actor.GetActorForwardVector` _returnvalue) (!= _returnvalue_2 (0.0 0.0 0.0)))))
    (:`CastFailed`
      (return (0.0 0.0 0.0)))))

(fn `GetMaxSpeed`
  (returns (MaxSpeed :type "Float (single-precision)"))
  (bind _aspawn (cast `Pawn` (`self.GetAvatarActorFromActorInfo`))
    (:`then`
      (return (`MovementComponent.GetMaxSpeed` (`Pawn.GetMovementComponent` _aspawn))))
    (:`CastFailed`
      (return 0.0))))