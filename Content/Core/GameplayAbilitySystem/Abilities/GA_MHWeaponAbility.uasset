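; Base gameplay ability for weapon abilities that can activate only while a specific weapon class is equipped.
; CanActivateAbility reads the avatar's BP_WeaponManager_Component and requires the EquippedWeapon class to exactly match RequiredWeaponEquipped.
; IsRequiredWeaponEquippedByActor repeats the same validity-checked test for any given actor.
; Activate and End events are empty, so this asset holds only the weapon gate.
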(fn `IsRequiredWeaponEquippedByActor`
  (params (Actor :type "Actor Object Reference"))
  (returns (ReturnValue :type Boolean))
  (bind _returnvalue (`Actor.GetComponentByClass` Actor "/Game/Core/Weapon/BP_WeaponManager_Component.BP_WeaponManager_Component_C"))
  (bind _equippedweapon (`/Game/Core/Weapon/BP_WeaponManager_Component.EquippedWeapon` _returnvalue))
  (`/Engine/EditorBlueprintResources/StandardMacros.IsValid` Actor
    (:`Is Valid`
      (`/Engine/EditorBlueprintResources/StandardMacros.IsValid` _returnvalue
        (:`Is Valid`
          (`/Engine/EditorBlueprintResources/StandardMacros.IsValid` _equippedweapon
            (:`Is Valid`
              (if (== (`self.RequiredWeaponEquipped`) (`GameplayStatics.GetObjectClass` _equippedweapon))
                (return true)
                (else
                  _)))
            (:`Is Not Valid`
              _)))
        (:`Is Not Valid`
          _)))
    (:`Is Not Valid`
      _))
  (return false))

(fn `K2_CanActivateAbility`
  (params (ActorInfo :type "GameplayAbilityActorInfo Structure") (Handle :type "GameplayAbilitySpecHandle Structure"))
  (returns (RelevantTags :type "GameplayTagContainer Structure") (ReturnValue :type Boolean))
  (bind (_owneractor _avataractor) (break `GameplayAbilityActorInfo` ActorInfo))
  (bind _returnvalue (`Actor.GetComponentByClass` _avataractor "/Game/Core/Weapon/BP_WeaponManager_Component.BP_WeaponManager_Component_C"))
  (bind _equippedweapon (`/Game/Core/Weapon/BP_WeaponManager_Component.EquippedWeapon` _returnvalue))
  (bind _returnvalue_2 (== (`self.RequiredWeaponEquipped`) (`GameplayStatics.GetObjectClass` _equippedweapon)))
  (`/Engine/EditorBlueprintResources/StandardMacros.IsValid` _avataractor
    (:`Is Valid`
      (`/Engine/EditorBlueprintResources/StandardMacros.IsValid` _returnvalue
        (:`Is Valid`
          (`/Engine/EditorBlueprintResources/StandardMacros.IsValid` _equippedweapon
            (:`Is Valid`
              (if _returnvalue_2
                (return (struct) _returnvalue_2)))
            (:`Is Not Valid`
              (return (struct) false))))
        (:`Is Not Valid`
          (return (struct) false))))
    (:`Is Not Valid`
      (return (struct) false))))