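; Base reactive gameplay ability that triggers a status effect when a debuff it applies to a target reaches maximum stacks.
; It listens for effects applied to targets, checking the debuff tag and stack count against its StatusEffectDataAsset.
; At the threshold, it builds the asset's effect spec, passes it through ModifyEffectSpec for a fixed set-by-caller damage magnitude, and applies it to that target.
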(event `self.K2_ActivateAbility`
  (bind _statuseffectdataasset (`self.StatusEffectDataAsset`))
  (bind _returnvalue (`self.MakeOutgoingGameplayEffectSpec` (`/Game/Core/GameplayAbilitySystem/Data/PDA_StatusEffect.GameplayEffectClass` _statuseffectdataasset)))
  (bind (_asynctaskproxy _target _spechandle _activehandle) (`AbilityTask_WaitGameplayEffectApplied_Target.WaitGameplayEffectAppliedToTarget` (struct) (struct) (struct) (struct) (struct) false null)
    (:`OnApplied`
      (bind _returnvalue_2 (`AbilitySystemBlueprintLibrary.GetGameplayEffectFromActiveEffectHandle` _activehandle))
      (`/Engine/EditorBlueprintResources/StandardMacros.IsValid` _returnvalue_2
        (:`Is Valid`
          (if (`GameplayTagAssetInterface.HasMatchingGameplayTag` _returnvalue_2 (`/Game/Core/GameplayAbilitySystem/Data/PDA_StatusEffect.DebuffTag` (`self.StatusEffectDataAsset`)))
            (bind _returnvalue_3 (`AbilitySystemBlueprintLibrary.GetActiveGameplayEffectStackCount` _activehandle))
            (if (>= _returnvalue_3 (`/Game/Core/GameplayAbilitySystem/Data/PDA_StatusEffect.MaxStackCount` _statuseffectdataasset))
              (`AbilitySystemBlueprintLibrary.SetDuration` _returnvalue (`/Game/Core/GameplayAbilitySystem/Data/PDA_StatusEffect.StatusDuration` _statuseffectdataasset))
              (bind _specout (`self.ModifyEffectSpec` _returnvalue))
              (`self.K2_ApplyGameplayEffectSpecToTarget` _specout (`AbilitySystemBlueprintLibrary.AbilityTargetDataFromActor` _target)))))))))

(fn `ModifyEffectSpec`
  (params (SpecIn :type "GameplayEffectSpecHandle Structure"))
  (returns (SpecOut :type "GameplayEffectSpecHandle Structure"))
  (bind _returnvalue (`AbilitySystemBlueprintLibrary.AssignTagSetByCallerMagnitude` SpecIn (struct :`TagName` "Data.Damage") 10.0))
  (return _returnvalue))