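; Gameplay ability for a staff area-of-effect lightning strike at a ground location.
; It uses the avatar's attack target ground point if one exists, otherwise player-controlled avatars pick a spot with a decal ground-trace target actor during a looping cast montage.
; After commit, a montage event fires the lightning cue inside an indicator cue.
; Following a short delay, the authority sphere-traces pawns and applies SetByCaller damage once per actor.
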(event `self.K2_ActivateAbility`
  ; Phase 1
  (bind _attacktarget (message `/Game/Core/Interface/BPI_Targeting.GetAttackTarget` (`self.GetAvatarActorFromActorInfo`)))
  (`/Engine/EditorBlueprintResources/StandardMacros.IsValid` _attacktarget
    (:`Is Valid`
      (bind _location (`self.GetTargetGroundLocation` _attacktarget))
      (set `self.ConfirmedAOELocation` _location)
      (`self.ConfirmStrike`))
    (:`Is Not Valid`
      (`self.StartTargeting`))))

(event `StartTargeting`
  ; Phase 1
  (if (`self.HasPlayerController`)
    (`self.LoopTargetingAnimaton`)
    (set `self.IsWaitingTargetData` true)
    (bind (_asynctaskproxy _data) (`AbilityTask_WaitTargetData.WaitTargetData` "None" "UserConfirmed" "/Game/Core/GameplayAbilitySystem/TargetingActors/GA_TA_GroundTrace_Decal.GA_TA_GroundTrace_Decal_C" (* (`self.AOERadius`) 2.0) "/Engine/EngineMaterials/DefaultDeferredDecalMaterial.DefaultDeferredDecalMaterial" 0.0 0.0 999999.0 (struct :`Name` "NoCollision") true (`self.MakeTargetLocationInfoFromOwnerActor`) (struct) null)
      (:`ValidData`
        (set `self.IsWaitingTargetData` false)
        (set `self.ConfirmedAOELocation` (`.Location` (`GameplayStatics.BreakHitResult` (`AbilitySystemBlueprintLibrary.GetHitResultFromTargetData` _data))))
        (`self.ConfirmStrike`)))
    (else
      (`self.K2_EndAbility`))))

(event `ConfirmStrike`
  ; Phase 2
  (bind _returnvalue (`self.K2_CommitAbility`))
  (if _returnvalue
    (set `self.IsFiring` true)
    (`self.K2_AddGameplayCueWithParams` (struct :`TagName` "GameplayCue.AOEIndicator") (`AbilitySystemBlueprintLibrary.MakeGameplayCueParameters` 0.0 (* (`self.AOERadius`) 2.0) (struct) (struct) (struct) (struct) (struct) (`self.ConfirmedAOELocation`)))
    (`AbilityTask_PlayMontageAndWait.CreatePlayMontageAndWaitProxy` "None" "/Game/Core/Animation/Manny/Staff/AS_Manny_Staff_skill3_Montage.AS_Manny_Staff_skill3_Montage"
      (:`then`
        (`AbilityTask_WaitGameplayEvent.WaitGameplayEvent` (struct :`TagName` "Event.Montage.Trigger") null
          (:`EventReceived`
            (`self.K2_ExecuteGameplayCueWithParams` (struct :`TagName` "GameplayCue.LightningBolt") (`AbilitySystemBlueprintLibrary.MakeGameplayCueParameters` 0.0 0.0 (struct) (struct) (struct) (struct) (struct) (`self.ConfirmedAOELocation`)))
            (`KismetSystemLibrary.Delay` 0.7)
            (`self.AOEDamage`)
            (`self.K2_RemoveGameplayCue` (struct :`TagName` "GameplayCue.AOEIndicator")))))
      (:`OnCompleted`
        (`self.K2_EndAbility` :!label _label)
        (set `self.IsFiring` false))
      (:`OnInterrupted`
        (goto _label)))
    (else
      (`self.K2_EndAbility`)
      (set `self.IsFiring` false))))

(event `LoopTargetingAnimaton`
  ; Phase 1
  (`AbilityTask_PlayMontageAndWait.CreatePlayMontageAndWaitProxy` "None" "/Game/Core/Animation/Manny/Staff/AS_Manny_Staff_CastingLoop_Montage.AS_Manny_Staff_CastingLoop_Montage"
    (:`OnBlendOut`
      (if (`self.IsWaitingTargetData`)
        (`self.LoopTargetingAnimaton`)))
    (:`OnInterrupted`
      (if (`self.IsWaitingTargetData`)
        (`self.K2_EndAbility`)))))

(event `AOEDamage`
  (bind _confirmedaoelocation (`self.ConfirmedAOELocation`))
  (bind _hitactors (`self.HitActors`))
  ; Phase 2
  (`self.K2_HasAuthority`
    (:`True`
      (bind _outhits (`KismetSystemLibrary.SphereTraceMultiForObjects` _confirmedaoelocation _confirmedaoelocation (`self.AOERadius`) (`|MakeArray` "ObjectTypeQuery3" :!type "EObjectTypeQuery Enum") false (`|MakeArray` (`self.GetAvatarActorFromActorInfo`)) "ForDuration"))
      (`KismetArrayLibrary.Array_Clear` (`self.HitActors`))
      (for _array_element _outhits
        (bind (_bblockinghit _binitialoverlap _time _distance _location _impactpoint _normal _impactnormal _physmat _hitactor) (`GameplayStatics.BreakHitResult` _array_element))
        (if (not (`KismetArrayLibrary.Array_Contains` _hitactors _hitactor))
          (`KismetArrayLibrary.Array_AddUnique` _hitactors _hitactor)
          (bind _returnvalue (`AbilitySystemBlueprintLibrary.GetAbilitySystemComponent` _hitactor))
          (`/Engine/EditorBlueprintResources/StandardMacros.IsValid` _returnvalue
            (:`Is Valid`
              (bind _returnvalue_2 (`AbilitySystemBlueprintLibrary.AssignTagSetByCallerMagnitude` (`self.MakeOutgoingGameplayEffectSpec` "/Game/Core/GameplayAbilitySystem/Effects/GE_Damage_Instant.GE_Damage_Instant_C") (struct :`TagName` "Data.Damage") (`self.DamageMagnitude`)))
              (`AbilitySystemComponent.BP_ApplyGameplayEffectSpecToTarget` (`AbilitySystemBlueprintLibrary.GetAbilitySystemComponent` (`self.GetAvatarActorFromActorInfo`)) _returnvalue_2 _returnvalue))))))))

(fn `GetTargetGroundLocation`
  (params (AttackTarget :type "Actor Object Reference"))
  (returns (Location :type "Vector Structure") (ReturnValue :type Boolean))
  (bind _returnvalue (`Actor.K2_GetActorLocation` AttackTarget))
  (bind (_outhit _returnvalue_2) (`KismetSystemLibrary.LineTraceSingle` _returnvalue (- _returnvalue (0.0 0.0 9999.0)) "TraceTypeQuery1" false (`|MakeArray` AttackTarget)))
  (return (`.Location` (`GameplayStatics.BreakHitResult` _outhit)) _returnvalue_2))