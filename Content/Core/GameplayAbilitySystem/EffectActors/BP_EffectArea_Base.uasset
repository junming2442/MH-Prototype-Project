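; Base effect area actor that applies a configurable Gameplay Effect to overlapping actors that have an Ability System Component.
; On begin overlap it builds a spec with itself as causer, sets a tagged SetByCaller magnitude and applies it to that actor.
; On end overlap it removes all stacks of that effect class, with no source filter specified.
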(event `self.ReceiveActorBeginOverlap`
  (params (OtherActor :type "Actor Object Reference"))
  (bind _returnvalue (`AbilitySystemBlueprintLibrary.GetAbilitySystemComponent` OtherActor))
  (`/Engine/EditorBlueprintResources/StandardMacros.IsValid` _returnvalue
    (:`Is Valid`
      (bind _returnvalue_2 (`AbilitySystemBlueprintLibrary.MakeSpecHandleByClass` (`self.GameplayEffectClass`) null self))
      (bind _returnvalue_3 (`AbilitySystemBlueprintLibrary.AssignTagSetByCallerMagnitude` _returnvalue_2 (`self.MagnitudeDataTag`) (`self.Magnitude`)))
      (`AbilitySystemComponent.BP_ApplyGameplayEffectSpecToSelf` _returnvalue _returnvalue_3))))

(event `self.ReceiveActorEndOverlap`
  (params (OtherActor :type "Actor Object Reference"))
  (bind _returnvalue (`AbilitySystemBlueprintLibrary.GetAbilitySystemComponent` OtherActor))
  (`/Engine/EditorBlueprintResources/StandardMacros.IsValid` _returnvalue
    (:`Is Valid`
      (`AbilitySystemComponent.RemoveActiveGameplayEffectBySourceEffect` _returnvalue (`self.GameplayEffectClass`) null -1))))

(fn `UserConstructionScript`)