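; Talent tree component that grants and upgrades an owning MH character's talents by spending talent points.
; Server_UpgradeTalent grants an unowned talent at level one or upgrades an owned one, checking points and max level, then deducts the cost.
; Grants add abilities and gameplay effects, storing handles per talent so upgrades can change their levels in place.
; RepNotifies on granted talents and remaining points fire update events.
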(event `self.ReceiveBeginPlay`
  (bind _returnvalue (`self.GetOwner`))
  (`/Engine/EditorBlueprintResources/StandardMacros.IsValid` _returnvalue
    (:`Is Valid`
      (bind _asmhcharacter_base (cast `MHCharacterBase` _returnvalue))
      (set `self.OwnerCharacter` _asmhcharacter_base)
      (`/Engine/EditorBlueprintResources/StandardMacros.IsValid` _returnvalue
        (:`Is Valid`
          (set `self.OwnerASC` (`AbilitySystemBlueprintLibrary.GetAbilitySystemComponent` _returnvalue)))))))

(event `Server_UpgradeTalent`
  (params (Talent :type "/Game/Core/GameplayAbilitySystem/Talents/PDA_Talent Object Reference"))
  (bind (_grantedtalent _isgranted) (`self.IsTalentGranted` Talent))
  (if _isgranted
    (bind _issuccess (`self.UpgradeTalent` _grantedtalent))
    (if _issuccess
      (`self.UseTalentPoints` (`/Game/Core/GameplayAbilitySystem/Talents/PDA_Talent.PointsRequired` Talent) :!label _label))
    (else
      (bind _issuccess_2 (`self.GrantTalent` Talent 1))
      (if _issuccess_2
        (goto _label)))))

(fn `ApplyGameplayEffectsFromTalentToOwner`
  (params (Talent :type "/Game/Core/GameplayAbilitySystem/Talents/PDA_Talent Object Reference (by ref)") (GameplayEffects :type "Array of GameplayEffect Class Reference") (Level :type Integer))
  (locals (AppliedEffectHandles :type "Array of ActiveGameplayEffectHandle Structure"))
  (bind _appliedeffecthandles (`local.AppliedEffectHandles`))
  (for _array_element GameplayEffects
    (bind _returnvalue (`AbilitySystemComponent.BP_ApplyGameplayEffectToSelf` :`self` (`self.OwnerASC`) :`GameplayEffectClass` _array_element :`Level` (`KismetMathLibrary.Conv_IntToDouble` Level)))
    (`KismetArrayLibrary.Array_AddUnique` _appliedeffecthandles _returnvalue)
    (`BlueprintMapLibrary.Map_Add` (`self.EffectHandleMap`) Talent (make `/Game/Core/GameplayAbilitySystem/Talents/F_TalentEffectHandle` _appliedeffecthandles))))

(fn `CanGrantTalent`
  (params (Talent :type "/Game/Core/GameplayAbilitySystem/Talents/PDA_Talent Object Reference"))
  (returns (ReturnValue :type Boolean) (ReturnMessage :type Text))
  (bind (_returnvalue _returnmessage) (`self.HasEnoughTalentPoints` (`/Game/Core/GameplayAbilitySystem/Talents/PDA_Talent.PointsRequired` Talent)))
  (if _returnvalue
    (return true "")
    (else
      (return false _returnmessage))))

(fn `CanUpgradeTalent`
  (params (GrantedTalent :type "/Game/Core/GameplayAbilitySystem/Talents/F_GrantedTalent Structure (by ref)"))
  (returns (ReturnValue :type Boolean) (ReturnMessage :type Text))
  (bind (_talent _currentlevel) (break `/Game/Core/GameplayAbilitySystem/Talents/F_GrantedTalent` GrantedTalent))
  (if (> (`/Game/Core/GameplayAbilitySystem/Talents/PDA_Talent.MaxLevel` _talent) _currentlevel)
    (bind (_returnvalue _returnmessage) (`self.HasEnoughTalentPoints` (`/Game/Core/GameplayAbilitySystem/Talents/PDA_Talent.PointsRequired` _talent)))
    (if _returnvalue
      (return true "")
      (else
        (return false _returnmessage)))
    (else
      (return false "Talent is at max level"))))

(fn `GrantAbilitiesFromTalentToOwner`
  (params (Talent :type "/Game/Core/GameplayAbilitySystem/Talents/PDA_Talent Object Reference (by ref)") (Abilities :type "Array of GameplayAbility Class Reference") (Level :type Integer))
  (bind _returnvalue (`MHCharacterBase.GrantAbilities` (`self.OwnerCharacter`) Abilities Level))
  (`BlueprintMapLibrary.Map_Add` (`self.AbilitySpecHandleMap`) Talent (make `/Game/Core/GameplayAbilitySystem/Talents/F_TalentAbilitySpecHandle` _returnvalue)))

(fn `GrantTalent`
  (params (Talent :type "/Game/Core/GameplayAbilitySystem/Talents/PDA_Talent Object Reference") (StartingLevel :type Integer))
  (returns (IsSuccess :type Boolean))
  (locals (ClampedLevel :type Integer))
  (bind _grantedtalents (`self.GrantedTalents`))
  (bind _clampedlevel (`local.ClampedLevel`))
  (bind _talent (`local.Talent`))
  (bind (_returnvalue _returnmessage) (`self.CanGrantTalent` Talent))
  (if _returnvalue
    (set `local.ClampedLevel` (`KismetMathLibrary.Clamp` StartingLevel 1 (`/Game/Core/GameplayAbilitySystem/Talents/PDA_Talent.MaxLevel` Talent)))
    (`self.GrantAbilitiesFromTalentToOwner` Talent (`/Game/Core/GameplayAbilitySystem/Talents/PDA_Talent.AbilitiesToGrant` Talent) _clampedlevel)
    (`self.ApplyGameplayEffectsFromTalentToOwner` _talent (`/Game/Core/GameplayAbilitySystem/Talents/PDA_Talent.EffectsToApply` _talent) _clampedlevel)
    (`KismetArrayLibrary.Array_Add` _grantedtalents (make `/Game/Core/GameplayAbilitySystem/Talents/F_GrantedTalent` (`local.Talent`) _clampedlevel))
    (set `self.GrantedTalents` _grantedtalents)
    (return true)
    (else
      (`KismetSystemLibrary.PrintString` (`KismetTextLibrary.Conv_TextToString` _returnmessage))
      (return false))))

(fn `HasEnoughTalentPoints`
  (params (PointsRequired :type Integer))
  (returns (ReturnValue :type Boolean) (ReturnMessage :type Text))
  (if (>= (`self.TalentPointsLeft`) PointsRequired)
    (return true "")
    (else
      (return false "Not enough talent points"))))

(fn `IsTalentGranted`
  (params (Talent :type "/Game/Core/GameplayAbilitySystem/Talents/PDA_Talent Object Reference"))
  (returns (GrantedTalent :type "/Game/Core/GameplayAbilitySystem/Talents/F_GrantedTalent Structure") (IsGranted :type Boolean))
  (for _array_element (`self.GrantedTalents`)
    (if (== (`.Talent_3_F5C809FE4B010F2CC24BCA92C1E96B13` (break `/Game/Core/GameplayAbilitySystem/Talents/F_GrantedTalent` _array_element)) Talent)
      (return _array_element true)))
  (return (struct) false))

(fn `OnRep_GrantedTalents`
  (`self.OnTalentsUpdated`))

(fn `OnRep_TalentPointsLeft`
  (`self.OnTalentPointsUpdated`))

(fn `UpgradeTalent`
  (params (GrantedTalent :type "/Game/Core/GameplayAbilitySystem/Talents/F_GrantedTalent Structure"))
  (returns (IsSuccess :type Boolean))
  (bind (_grantedtalent_talent _grantedtalent_currentlevel) (break `/Game/Core/GameplayAbilitySystem/Talents/F_GrantedTalent` (`local.GrantedTalent`)))
  (bind (_grantedtalent_talent_2 _grantedtalent_currentlevel_2) (break `/Game/Core/GameplayAbilitySystem/Talents/F_GrantedTalent` (`local.GrantedTalent`)))
  (bind _grantedtalent_talent_3 (break `/Game/Core/GameplayAbilitySystem/Talents/F_GrantedTalent` (`local.GrantedTalent`)))
  (bind (_grantedtalent_talent_4 _grantedtalent_currentlevel_3) (break `/Game/Core/GameplayAbilitySystem/Talents/F_GrantedTalent` (`local.GrantedTalent`)))
  (bind _grantedtalents (`self.GrantedTalents`))
  (bind _grantedtalent_talent_5 (break `/Game/Core/GameplayAbilitySystem/Talents/F_GrantedTalent` (`local.GrantedTalent`)))
  (bind _returnvalue (`KismetArrayLibrary.Array_Find` _grantedtalents GrantedTalent))
  (bind (_returnvalue_2 _returnmessage) (`self.CanUpgradeTalent` GrantedTalent))
  (if _returnvalue_2
    ; Upgrade Talent Level
    (if (`KismetArrayLibrary.Array_IsValidIndex` _grantedtalents _returnvalue)
      (`KismetArrayLibrary.Array_Set` _grantedtalents _returnvalue (make `/Game/Core/GameplayAbilitySystem/Talents/F_GrantedTalent` _grantedtalent_talent_4 (+ _grantedtalent_currentlevel_3 (`self.LevelToAdd`))))
      (set `self.GrantedTalents` _grantedtalents)
      (`|ExecutionSequence`
        (:`then_0`
          ; Upgrade GameplayEffects
          (for _array_element (break `/Game/Core/GameplayAbilitySystem/Talents/F_TalentEffectHandle` (`BlueprintMapLibrary.Map_Find` (`self.EffectHandleMap`) _grantedtalent_talent_5))
            (`AbilitySystemComponent.SetActiveGameplayEffectLevel` (`self.OwnerASC`) _array_element (+ _grantedtalent_currentlevel_2 (`self.LevelToAdd`)))))
        (:`then_1`
          ; Upgrade GameplayAbilities
          (for _array_element_2 (break `/Game/Core/GameplayAbilitySystem/Talents/F_TalentAbilitySpecHandle` (`BlueprintMapLibrary.Map_Find` (`self.AbilitySpecHandleMap`) _grantedtalent_talent_3))
            (bind _asmhgameplay_ability (cast `MHGameplayAbility` (`.ReturnValue` (`AbilitySystemBlueprintLibrary.GetGameplayAbilityFromSpecHandle` (`self.OwnerASC`) _array_element_2))))
            (`MHGameplayAbility.SetAbilityLevel` _asmhgameplay_ability (+ _grantedtalent_currentlevel (`self.LevelToAdd`)))))
        (:`then_2`
          (return true))))
    (else
      (`KismetSystemLibrary.PrintString` (`KismetTextLibrary.Conv_TextToString` _returnmessage))
      (return false))))

(fn `UseTalentPoints`
  (params (Points :type Integer))
  (set `self.TalentPointsLeft` (- (`self.TalentPointsLeft`) Points)))