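; Base enemy character built on the Gameplay Ability System, exposing combat, patrol and movement functions for AI control.
; Attack sets AI focus and activates a random ability matching its type tag, and ability end signals that attacking finished.
; Weapon equip fires a gameplay event, while UnequipWeapon is empty.
; A vitals widget is created on BeginPlay and removed on death, and movement states scale the cached default walk speed.
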(event `self.ReceiveBeginPlay`
  (bind _returnvalue (`|CreateWidget` "/Game/Core/Widgets/Enemy/WBP_EnemyVitals.WBP_EnemyVitals_C" null self))
  (`WidgetComponent.SetWidget` (`self.HealthBarWidget`) _returnvalue)
  (set `self.DefaultWalkSpeed` (`CharacterMovementComponent.MaxWalkSpeed` (`self.CharacterMovement`))))

(event `self.ReceivePossessed`
  (params (NewController :type "Controller Object Reference"))
  (`KismetSystemLibrary.DelayUntilNextTick`))

(event `Attack`
  (params (AttackTarget :type "Actor Object Reference"))
  (`/Game/Core/Interface/BPI_Targeting.GetAttackTarget`)
  (`AIController.K2_SetFocus` (`AIBlueprintHelperLibrary.GetAIController` self) AttackTarget)
  (bind _outabilityhandles (`AbilitySystemComponent.FindAllAbilitiesWithTags` (`self.AbilitySystemComponent`) (`self.AbilityTypeTag`) false))
  (`AbilitySystemComponent.TryActivateAbility` (`self.AbilitySystemComponent`) (`KismetArrayLibrary.Array_Random` _outabilityhandles) true))

(event `self.HandleAbilityEnded`
  (params (AbilityEndedData :type "AbilityEndedData Structure (by ref)"))
  (`self.OnFinishAttacking`))

(event `self.HandleDeath`
  (`parent.HandleDeath`)
  (bind _healthbarwidget (`self.HealthBarWidget`)
    (:`then`
      (`ActorComponent.K2_DestroyComponent` _healthbarwidget))
    (:`else`)))

(event `/Game/Core/Enemy/BPI_EnemyAI.EquipWeapon`
  (`AbilitySystemBlueprintLibrary.SendGameplayEventToActor` self (struct :`TagName` "Event.ActivateAbility.EquipWeapon") (make `GameplayEventData` (struct) null null null null (struct) (struct) (`self.WeaponTypeTag`))))

(event `/Game/Core/Enemy/BPI_EnemyAI.UnequipWeapon`)

(fn `GetAttackTarget`
  (returns (AttackTarget :type "Actor Object Reference"))
  (bind _returnvalue (`AIController.GetFocusActor` (`AIBlueprintHelperLibrary.GetAIController` self)))
  (`/Engine/EditorBlueprintResources/StandardMacros.IsValid` _returnvalue
    (:`Is Valid`
      (return _returnvalue))))

(fn `GetIdealRange`
  (returns (AttackRadius :type "Float (double-precision)") (DefendRadius :type "Float (double-precision)"))
  (return 250.0 400.0))

(fn `GetPatrolRoute`
  (returns (PatrolRoute :type "/Game/Core/Enemy/BP_PatrolRoute Object Reference"))
  (return (`self.PatrolRoute`)))

(fn `SetMovementSpeed`
  (params (MovementState :type "/Game/Core/Enemy/Enums/Enum_MovementState Enum" :default "NewEnumerator0"))
  (returns (MovementSpeed :type "Float (double-precision)"))
  (bind _defaultwalkspeed (`self.DefaultWalkSpeed`))
  (bind _output_get (set `CharacterMovementComponent.MaxWalkSpeed` (select `/Game/Core/Enemy/Enums/Enum_MovementState` MovementState :`NewEnumerator3` (* _defaultwalkspeed 0.3) :`NewEnumerator1` (* _defaultwalkspeed 0.5) :`NewEnumerator2` (`self.DefaultWalkSpeed`) :!type "Float (single-precision)") (`self.CharacterMovement`)))
  (return _output_get))

(fn `UserConstructionScript`)