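; Base GAS enemy character Blueprint that shows a vitals widget and provides attack, range, patrol route and movement speed functions, apparently for AI.
; Attack focuses the AI controller on the target, activates a random melee combo ability found by tag, and reports completion when the ability ends.
; Movement states scale the walk speed cached at BeginPlay, and death removes the health bar.
; Equip, shield regen and armor test logic is disconnected.
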(event `self.ReceiveBeginPlay`
  (bind _returnvalue (`|CreateWidget` "/Game/Core/Widgets/Enemy/WBP_EnemyVitals.WBP_EnemyVitals_C" null self))
  (`WidgetComponent.SetWidget` (`self.HealthBarWidget`) _returnvalue)
  (set `self.DefaultWalkSpeed` (`CharacterMovementComponent.MaxWalkSpeed` (`self.CharacterMovement`))))

(event `self.ReceivePossessed`
  (params (NewController :type "Controller Object Reference"))
  (`KismetSystemLibrary.DelayUntilNextTick`))

(event `Attack`
  (params (AttackTarget :type "Actor Object Reference"))
  (`AIController.K2_SetFocus` (`AIBlueprintHelperLibrary.GetAIController` self) AttackTarget)
  (bind _outabilityhandles (`AbilitySystemComponent.FindAllAbilitiesWithTags` (`self.AbilitySystemComponent`) (struct :`GameplayTags` (struct :`(TagName` "GameplayAbility.MeleeAttack.Combo"))) true))
  (`AbilitySystemComponent.TryActivateAbility` (`self.AbilitySystemComponent`) (`KismetArrayLibrary.Array_Random` _outabilityhandles) true))

(event `self.HandleAbilityEnded`
  (params (AbilityEndedData :type "AbilityEndedData Structure (by ref)"))
  (`self.OnFinishAttacking`))

(event `self.HandleDeath`
  (`parent.HandleDeath`)
  (bind _healthbarwidget (`self.HealthBarWidget`)
    (:`then`
      (`ActorComponent.K2_DestroyComponent` _healthbarwidget))
    (:`else`)))

(fn `GetAttackTarget`
  (returns (AttackTarget :type "Actor Object Reference"))
  (return (`GameplayStatics.GetPlayerCharacter` 0)))

(fn `GetIdealRange`
  (returns (AttackRadius :type "Float (double-precision)") (DefendRadius :type "Float (double-precision)"))
  (return 250.0 400.0))

(fn `GetPatrolRoute`
  (returns (PatrolRoute :type "/Game/Core/Enemy/BP_PatrolRoute Object Reference"))
  (return (`self.PatrolRoute`)))

(fn `SetMovementSpeed`
  (params (MovementState :type "/Game/Core/Enemy/Enums/Enum_MovementState Enum" :default "NewEnumerator0"))
  (returns (MovementSpeed :type "Float (double-precision)"))
  (bind _defaultwalkspeed (`self.DefaultWalkSpeed`))
  (bind _output_get (set `CharacterMovementComponent.MaxWalkSpeed` (select `/Game/Core/Enemy/Enums/Enum_MovementState` MovementState :`NewEnumerator3` (* _defaultwalkspeed 0.3) :`NewEnumerator1` (* _defaultwalkspeed 0.5) :`NewEnumerator2` (`self.DefaultWalkSpeed`) :!type "Float (single-precision)") (`self.CharacterMovement`)))
  (return _output_get))

(fn `UserConstructionScript`)