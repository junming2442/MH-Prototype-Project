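; BP_Skill_FireProjectileExplo is a wizard fire skill actor that charges, launches a fireball and ends in an explosion.
; On BeginPlay it plays a charge effect, then after a timed delay swaps it for a small burst and spawns a BP_Wizard_Projectile with fireball visuals.
; A second fixed delay, just short of the projectile's lifetime, spawns the large explosion slightly below the projectile's position, with no hit detection here.
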(event `self.ReceiveBeginPlay`
  (bind _returnvalue (`NiagaraFunctionLibrary.SpawnSystemAtLocation` "/Game/Wizard/Particles/Fire/PS_FireBall_Charge.PS_FireBall_Charge" (`self.K2_GetActorLocation` self)))
  (`KismetSystemLibrary.Delay` 3.0)
  (`ActorComponent.K2_DestroyComponent` _returnvalue)
  (`NiagaraFunctionLibrary.SpawnSystemAtLocation` "/Game/Wizard/Particles/Fire/PS_Fire_explosion_small.PS_Fire_explosion_small" (`self.K2_GetActorLocation` self))
  (bind _returnvalue_2 (`|SpawnActorFromClass` "/Game/Wizard/Blueprints/BP_Wizard_Projectile.BP_Wizard_Projectile_C" (`KismetMathLibrary.MakeTransform` (`self.K2_GetActorLocation` self)) "Undefined" "OverrideRootScale" null 650.0 1.5 "/Game/Wizard/Particles/Fire/PS_FireBall_Projectile.PS_FireBall_Projectile" null))
  (`KismetSystemLibrary.Delay` 1.45)
  (bind (_returnvalue_x _returnvalue_y _returnvalue_z) (`KismetMathLibrary.BreakVector` (`self.K2_GetActorLocation` _returnvalue_2)))
  (`NiagaraFunctionLibrary.SpawnSystemAtLocation` "/Game/Wizard/Particles/Fire/PS_Fire_explosion.PS_Fire_explosion" (`KismetMathLibrary.MakeVector` _returnvalue_x _returnvalue_y (- _returnvalue_z 100.0))))

(fn `UserConstructionScript`)