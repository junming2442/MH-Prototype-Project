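; BP_Wizard_MeteroidProj is the wizard's meteor projectile actor, moved by a ProjectileMovement component whose initial speed comes from a Speed variable at construction.
; On BeginPlay it assigns a projectile Niagara system to its effect component.
; When its sphere collider hits something, it spawns a meteor fire explosion, hides the meteorite mesh, stops sphere physics and destroys itself after a short delay.
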(event `self.ReceiveBeginPlay`
  (`NiagaraComponent.SetAsset` (`self.Niagara`) (`self.Projectile`) true))

(event `self.Sphere.OnComponentHit`
  (params (HitComponent :type "PrimitiveComponent Object Reference") (OtherActor :type "Actor Object Reference") (OtherComp :type "PrimitiveComponent Object Reference") (NormalImpulse :type "Vector Structure") (Hit :type "HitResult Structure (by ref)"))
  (`NiagaraFunctionLibrary.SpawnSystemAtLocation` "/Game/Wizard/Particles/Fire/PS_Fire_Explosion_Meteor.PS_Fire_Explosion_Meteor" (`self.K2_GetActorLocation` self))
  (`SceneComponent.SetVisibility` (`self.SM_meteroite`) false false)
  (`PrimitiveComponent.SetSimulatePhysics` (`self.Sphere`) false)
  (`KismetSystemLibrary.Delay` 2.0)
  (`self.K2_DestroyActor` self))

(fn `UserConstructionScript`
  (set `ProjectileMovementComponent.InitialSpeed` (`self.Speed`) (`self.ProjectileMovement`)))