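; BP_Wizard_Projectile is a wizard projectile actor with a configurable Niagara visual, speed and lifetime.
; The construction script copies Speed into the ProjectileMovement component's initial speed.
; On BeginPlay it assigns the Projectile effect to its Niagara component, then destroys itself after LifeTime elapses.
; The file shows no hit or damage logic.
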(event `self.ReceiveBeginPlay`
  (`NiagaraComponent.SetAsset` (`self.Niagara`) (`self.Projectile`) true)
  (`KismetSystemLibrary.Delay` (`self.LifeTime`))
  (`self.K2_DestroyActor` self))

(fn `UserConstructionScript`
  (set `ProjectileMovementComponent.InitialSpeed` (`self.Speed`) (`self.ProjectileMovement`)))